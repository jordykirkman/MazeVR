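; BP_PickupCube is a physics cube that BP_MotionController can pick up and drop, and that affects a Gate it hits.
; Pickup disables mesh collision and physics, then attaches the actor to the supplied component, keeping its world transform.
; Drop re-enables physics and detaches the cube but does not restore collision.
; Hitting a Gate sets that Gate's Cube component to a fixed raised relative location.
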(event EventBeginPlay)

(event Collision|EventHit
  (params (MyComp :type Primitive%20Component%20Object%20Reference) (Other :type Actor%20Object%20Reference) (OtherComp :type Primitive%20Component%20Object%20Reference) (bSelfMoved :type Boolean) (HitLocation :type Vector :default "0, 0, 0") (HitNormal :type Vector :default "0, 0, 0") (NormalImpulse :type Vector :default "0, 0, 0") (Hit :type Hit%20Result%20Structure%20%28by%20ref%29))
  (bind _asgate (Utilities|Casting|CastToGate Other))
  (Transformation|SetRelativeLocation (Variables|/Game/Blueprints/Gate.Gate_C|GetCube _asgate) "0, 0,50.000000" false false))

(event EventTick
  (params (DeltaSeconds :type Float%20%28single-precision%29)))

(event EventPickup
  (params (AttachTo :type Scene%20Component%20Object%20Reference))
  (Collision|SetCollisionEnabled (Variables|Debug|GetStaticMeshComponent) "NoCollision")
  (Physics|SetSimulatePhysics (Variables|Debug|GetStaticMeshComponent) false)
  (Transformation|AttachComponentToComponent (VehicleSound|GetRootComponent) AttachTo "None" "KeepWorld" "KeepWorld" "KeepWorld" false))

(event EventDrop
  (Physics|SetSimulatePhysics (Variables|Debug|GetStaticMeshComponent) true)
  (Transformation|DetachFromActor "KeepWorld" "KeepWorld" "KeepWorld"))

(fn ConstructionScript)
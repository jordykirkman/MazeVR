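; BP_PickupCube is a cube actor that a motion controller can pick up and drop.
; Pickup, called by BP_MotionController, disables the static mesh's collision and physics simulation, then attaches the root component to the given component, keeping world transform.
; Drop restores query and physics collision, re-enables simulation and detaches the actor in place.
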(event EventPickup
  (params (AttachTo :type Scene%20Component%20Object%20Reference))
  (Collision|SetCollisionEnabled (Variables|Debug|GetStaticMeshComponent) "NoCollision")
  (Physics|SetSimulatePhysics (Variables|Debug|GetStaticMeshComponent) false)
  (Transformation|AttachComponentToComponent (VehicleSound|GetRootComponent) AttachTo "None" "KeepWorld" "KeepWorld" "KeepWorld" false))

(event EventDrop
  (Collision|SetCollisionEnabled (Variables|Debug|GetStaticMeshComponent) "QueryAndPhysics")
  (Physics|SetSimulatePhysics (Variables|Debug|GetStaticMeshComponent) true)
  (Transformation|DetachFromActor "KeepWorld" "KeepWorld" "KeepWorld"))

(fn ConstructionScript)